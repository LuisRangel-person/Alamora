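; Buffalo enemy that charges in a straight line, moving along its mesh's forward axis each Tick without sweep and showing its health as text.
; Hitting a non-invincible player cuts health and armor, launches them against their velocity and calls GhostFrames.
; Any damage removes a fixed amount of health; at zero it destroys itself, lowers the player's remaining-enemy count and awards money.
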(event EventBeginPlay)

(event Collision|EventActorBeginOverlap
  (params (OtherActor :type Actor%20Object%20Reference)))

(event Game|Damage|EventAnyDamage
  (params (Damage :type Float%20%28single-precision%29) (DamageType :type Damage%20Type%20Object%20Reference) (InstigatedBy :type Controller%20Object%20Reference) (DamageCauser :type Actor%20Object%20Reference))
  ;[1 1 1] Getting Shot
  (Variables|Default|SetHealth (- (Variables|Default|GetHealth) 10))
  (if (<= (Variables|Default|GetHealth) 0)
    (Actor|DestroyActor)
    (bind _asthird_person_character (Utilities|Casting|CastToThirdPersonCharacter (Game|GetPlayerCharacter 0)))
    (Variables|/Game/ThirdPersonCPP/Blueprints/ThirdPersonCharacter.ThirdPersonCharacter_C|SetEnemies%20Remaining _asthird_person_character (- (Variables|/Game/ThirdPersonCPP/Blueprints/ThirdPersonCharacter.ThirdPersonCharacter_C|GetEnemies%20Remaining _asthird_person_character) 1))
    (Variables|/Game/ThirdPersonCPP/Blueprints/ThirdPersonCharacter.ThirdPersonCharacter_C|SetMoney _asthird_person_character (+ (Variables|/Game/ThirdPersonCPP/Blueprints/ThirdPersonCharacter.ThirdPersonCharacter_C|GetMoney _asthird_person_character) 25.0))))

(event EventTick
  (params (DeltaSeconds :type Float%20%28single-precision%29))
  (bind _mesh (Variables|Character|GetMesh))
  (bind _returnvalue (Transformation|GetWorldTransform _mesh))
  (bind (_location _rotation _scale) (Math|Transform|BreakTransform _returnvalue))
  ;[1 1 1] Movement
  (Transformation|SetActorTransform (Math|Transform|MakeTransform (+ _location (* (Math|Vector|Normalize (Math|Rotator|GetRotationXVector _rotation)) (* (Utilities|Time|GetWorldDeltaSeconds) (Variables|Default|GetSpeed)))) _rotation _scale))
  ;[1 1 1] Health Above Head
  (Rendering|Components|TextRender|SetText (Variables|Default|GetHealthRender) (Utilities|Text|ToText(Integer) (Variables|Default|GetHealth))))

(event Collision|EventHit
  (params (MyComp :type Primitive%20Component%20Object%20Reference) (Other :type Actor%20Object%20Reference) (OtherComp :type Primitive%20Component%20Object%20Reference) (bSelfMoved :type Boolean) (HitLocation :type Vector :default "0, 0, 0") (HitNormal :type Vector :default "0, 0, 0") (NormalImpulse :type Vector :default "0, 0, 0") (Hit :type Hit%20Result%20Structure%20%28by%20ref%29))
  (bind _force (Variables|Default|GetForce))
  ;[1 1 1] Collsion with Player
  (if (Actor|ActorHasTag Other "Player")
    (bind _asthird_person_character (Utilities|Casting|CastToThirdPersonCharacter (Game|GetPlayerCharacter 0)))
    (if (not (Variables|/Game/ThirdPersonCPP/Blueprints/ThirdPersonCharacter.ThirdPersonCharacter_C|GetInvincible _asthird_person_character))
      (Variables|/Game/ThirdPersonCPP/Blueprints/ThirdPersonCharacter.ThirdPersonCharacter_C|SetHealth _asthird_person_character (- (Variables|/Game/ThirdPersonCPP/Blueprints/ThirdPersonCharacter.ThirdPersonCharacter_C|GetHealth _asthird_person_character) 2e+01))
      (Variables|/Game/ThirdPersonCPP/Blueprints/ThirdPersonCharacter.ThirdPersonCharacter_C|SetArmor _asthird_person_character (- (Variables|/Game/ThirdPersonCPP/Blueprints/ThirdPersonCharacter.ThirdPersonCharacter_C|GetArmor _asthird_person_character) 1.0))
      (Character|LaunchCharacter _asthird_person_character (Math|Vector|MakeVector (* (.X (Math|Vector|BreakVector (Transformation|GetVelocity _asthird_person_character))) -1.0 _force) (* (.Y (Math|Vector|BreakVector (Transformation|GetVelocity _asthird_person_character))) -1.0 _force) (+ (* (.Z (Math|Vector|BreakVector (Transformation|GetVelocity _asthird_person_character))) 0.0) 2e+01)) true true)
      (Default|GhostFrames _asthird_person_character))))

(fn ConstructionScript)

(fn Movement)